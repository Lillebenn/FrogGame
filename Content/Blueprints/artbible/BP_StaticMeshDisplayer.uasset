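; Art bible display actor that shows meshes from a StaticMeshes array on its DisplayedObject component, starting at StartIndex.
; Tick applies the current mesh; with AutoDisplay on, a Delay inside Tick paces the advance through the array.
; At the end it wraps to the first mesh if ShouldLoop is set, otherwise holds the last.
; The index only advances past valid entries, so an empty slot stalls the cycle.
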(event EventBeginPlay
  (Variables|ArtDisplay|SetIndex (Variables|ArtDisplay|GetStartIndex)))

(event Collision|EventActorBeginOverlap
  (params (OtherActor :type Actor%20Object%20Reference)))

(event EventTick
  (params (DeltaSeconds :type Float%20%28single-precision%29))
  (bind _static_meshes (Variables|ArtDisplay|GetStatic%20Meshes))
  (if (Variables|ArtDisplay|GetAutoDisplay)
    (Utilities|FlowControl|Delay (Variables|ArtDisplay|GetDelay)))
  (Utilities|IsValid (Utilities|Array|Get(acopy) _static_meshes (Variables|ArtDisplay|GetIndex))
    (:Is%20Valid
      (Components|StaticMesh|SetStaticMesh (Variables|Default|GetDisplayedObject) (Utilities|Array|Get(acopy) _static_meshes (Variables|ArtDisplay|GetIndex)))
      (if (Variables|ArtDisplay|GetAutoDisplay)
        (Variables|ArtDisplay|SetIndex (+ (Variables|ArtDisplay|GetIndex) 1))
        (if (>= (Variables|ArtDisplay|GetIndex) (Utilities|Array|Length _static_meshes))
          (if (Variables|ArtDisplay|GetShouldLoop)
            (Variables|ArtDisplay|SetIndex 0)
            (else
              (Variables|ArtDisplay|SetIndex (- (Variables|ArtDisplay|GetIndex) 1)))))))))

(fn ConstructionScript)