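; Art bible actor that displays static meshes from the Bp_mesh_array actor, either fixed on one or cycling through them.
; On BeginPlay it finds that actor and copies the mesh of each of its StaticMeshComponents into an array.
; Tick sets DisplayedObject to the mesh at Index, which begins at StartIndex.
; With AutoDisplay on, a Delay inside Tick paces the index, which wraps to zero after the last mesh.
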(event EventBeginPlay
  (Variables|Default|SetIndex (Variables|Default|GetStartIndex))
  (bind _returnvalue (Actor|GetActorOfClass "/Game/Blueprints/artbible/bp_mesh_array.bp_mesh_array_C"))
  (bind _output_get (Variables|Default|SetMesh%20Array%20Actor _returnvalue))
  (Utilities|IsValid _output_get
    (:Is%20Valid
      (for (_ _array_index) (Actor|GetComponentsByClass (Variables|Default|GetMesh%20Array%20Actor) "/Script/Engine.StaticMeshComponent")
        (Utilities|Array|Add (Variables|Default|GetStatic%20Mesh%20Array) (Variables|/Script/Engine.StaticMeshComponent|GetStaticMesh (Utilities|Array|Get(acopy) (Actor|GetComponentsByClass (Variables|Default|GetMesh%20Array%20Actor) "/Script/Engine.StaticMeshComponent") _array_index)))))))

(event Collision|EventActorBeginOverlap
  (params (OtherActor :type Actor%20Object%20Reference)))

(event EventTick
  (params (DeltaSeconds :type Float%20%28single-precision%29))
  (bind _static_mesh_array (Variables|Default|GetStatic%20Mesh%20Array))
  (Utilities|IsValid (Variables|Default|GetMesh%20Array%20Actor)
    (:Is%20Valid
      (if (Variables|Default|GetAutoDisplay)
        (Utilities|FlowControl|Delay (Variables|Default|GetDelay)))
      (Utilities|IsValid (Utilities|Array|Get(acopy) _static_mesh_array (Variables|Default|GetIndex))
        (:Is%20Valid
          (Components|StaticMesh|SetStaticMesh (Variables|Default|GetDisplayedObject) (Utilities|Array|Get(acopy) _static_mesh_array (Variables|Default|GetIndex)))
          (if (Variables|Default|GetAutoDisplay)
            (Variables|Default|SetIndex (+ (Variables|Default|GetIndex) 1))
            (if (>= (Variables|Default|GetIndex) (Utilities|Array|Length _static_mesh_array))
              (Variables|Default|SetIndex 0))))))))

(fn ConstructionScript)