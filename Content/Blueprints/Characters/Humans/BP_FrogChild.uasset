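; BP_FrogChild is a collectible frog child character with an animated arrow that marks it in the world.
; On BeginPlay, a timeline drives the DirectionArrow's relative location, scale and rotation to make it bob, squash and spin.
; The timeline's Finished output checks IsCollected and, if true, stops the timeline and hides the arrow.
; The file only reads IsCollected and contains no collection logic.
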(event EventBeginPlay
  (bind _directionarrow (Variables|Default|GetDirectionArrow))
  ;[1 1 1] arrow loop anim
  (bind (_direction _position _scale _rotation _rotation_2) (Timeline|Timeline_0 PlayFromStart)
    (:Update
      (Transformation|SetRelativeLocation _directionarrow (Math|Vector|Lerp(Vector) "0, 0,400.000000" "0, 0,200.000000" _position) false false)
      (Transformation|SetRelativeScale3D _directionarrow (Math|Vector|Lerp(Vector) "1.000000,1.000000,1.000000" "1.200000,1.200000,0.800000" _scale))
      (Transformation|SetRelativeRotation _directionarrow (Math|Rotator|Lerp(Rotator) "0, 0, 0" "0.000000,360.000000,0.000000" _rotation) false false))
    (:Finished
      ;[1 1 1] Hide the Arrow and stop the timeline if the frog child is collected
      (if (Variables|Default|GetbIsCollected)
        (Utilities|FlowControl|Sequence
          (:then_0
            (Timeline|Timeline_0 Stop))
          (:then_1
            (Rendering|SetVisibility (Variables|Default|GetDirectionArrow) false false)))))))

(event Collision|EventActorBeginOverlap
  (params (OtherActor :type Actor%20Object%20Reference)))

(event EventTick
  (params (DeltaSeconds :type Float%20%28single-precision%29)))

(fn ConstructionScript)