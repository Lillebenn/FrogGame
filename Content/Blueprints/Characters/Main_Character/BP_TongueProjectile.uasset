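; Tongue projectile for the main character that retracts or drags an edible target, using timeline-driven lerps.
; The return timeline halts the projectile's velocity and moves it back through LerpMoveActor.
; The drag timeline moves the valid Target the same way, then destroys the EdibleMesh actor.
; Both timelines finish by calling RemoveCable on the ThirdPersonCharacter and destroying the projectile.
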(event EventStartReturnTimeline
  ;[1 1 1] Drags tongue back after a short delay
  (bind _lerpvalue (Timeline|Comeback Play)
    (:Update
      (Variables|/Script/Engine.MovementComponent|SetVelocity (Variables|Default|GetTongueProjectile) "0, 0, 0")
      (Class|TongueProjectile|LerpMoveActor self _lerpvalue))
    (:Finished
      (Class|FrogGameCharacter|RemoveCable (.AsThird%20Person%20Character (Utilities|Casting|CastToThirdPersonCharacter (Game|GetPlayerCharacter 0))))
      (Actor|DestroyActor))))

(event EventStartDragObjectTimeline
  (bind _target (Variables|Default|GetTarget))
  (bind _newtrack_0 (Timeline|Timeline_0 Play)
    (:Update
      (Utilities|IsValid _target
        (:Is%20Valid
          (Class|TongueProjectile|LerpMoveActor _target _newtrack_0))))
    (:Finished
      (Class|FrogGameCharacter|RemoveCable (.AsThird%20Person%20Character (Utilities|Casting|CastToThirdPersonCharacter (Game|GetPlayerCharacter 0))))
      (Utilities|FlowControl|Sequence
        (:then_0
          (Actor|DestroyActor (Variables|Default|GetEdible%20Mesh)))
        (:then_1
          (Actor|DestroyActor))))))

(fn ConstructionScript)