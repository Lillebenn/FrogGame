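; Main frog character Blueprint that implements a three-hit punch combo, available only in PowerMode.
; Punch input starts the montage or calls NextPunch, which cycles first punch, second punch and uppercut sections when CanPunch allows.
; Each hit clears CanPunch and restarts a Countdown timeline that drives ResetPunchDelay.
; Tick stops the montage and ends the combo once that delay runs out.
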(event Custom|NextPunch
  ;[1 1 1] Looping the punches
  (if (Variables|Default|GetCanPunch)
    (Variables|Default|SetResetPunchDelay 1.0)
    (switch Utilities|FlowControl|Switch|SwitchonPunchCombo (Variables|Default|GetCurrentPunch)
      (:NewEnumerator0
        (Animation|PlayAnimMontage "/Game/Models/Player/Player_Powered/PunchingMontage.PunchingMontage" 1.0 "Second Punch")
        (Variables|Default|SetCurrentPunch "NewEnumerator1"))
      (:NewEnumerator1
        (Animation|PlayAnimMontage "/Game/Models/Player/Player_Powered/PunchingMontage.PunchingMontage" 1.0 "UpperCut")
        (Variables|Default|SetCurrentPunch "NewEnumerator2"))
      (:NewEnumerator2
        (Animation|PlayAnimMontage "/Game/Models/Player/Player_Powered/PunchingMontage.PunchingMontage" 1.0 "First Punch")
        (Variables|Default|SetCurrentPunch "NewEnumerator0")))
    (Variables|Default|SetCanPunch false)
    (bind _countdown (Timeline|Countdown PlayFromStart)
      (:Update
        (Variables|Default|SetResetPunchDelay _countdown)))))

(event EventTick
  (params (DeltaSeconds :type Float%20%28single-precision%29))
  (bind _mesh (Variables|Character|GetMesh))
  (bind _returnvalue (Components|SkeletalMesh|GetAnimInstance _mesh))
  (if (<= (Variables|Default|GetResetPunchDelay) 0.0)
    (Utilities|IsValid _returnvalue
      (:Is%20Valid
        (Animation|Montage|MontageStop _returnvalue 0.0 "/Game/Models/Player/Player_Powered/PunchingMontage.PunchingMontage"))
      (:Is%20Not%20Valid
        _))
    (Variables|Default|SetIsPunching false)))

(event Input|ActionEvents|InputActionPunch
  (params (Key :type Key%20Structure :default "None"))
  ;[1 1 1] Punching
  (:Pressed
    (if (Variables|Default|GetbPowerMode)
      (if (Variables|Default|GetIsPunching)
        (CallFunction|NextPunch)
        (else
          (Variables|Default|SetIsPunching true)
          (Animation|Montage|MontagePlay (Components|SkeletalMesh|GetAnimInstance (Variables|Character|GetMesh)) "/Game/Models/Player/Player_Powered/PunchingMontage.PunchingMontage" 1.0 "MontageLength" 0.0 true)
          (Variables|Default|SetCurrentPunch "NewEnumerator0")
          ;[1 1 1] Looping the punches
          (Variables|Default|SetCanPunch false)
          (bind _countdown (Timeline|Countdown PlayFromStart)
            (:Update
              (Variables|Default|SetResetPunchDelay _countdown))))))))

(fn ConstructionScript)