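; Enemy animal Blueprint that gives its CreatureMesh procedural idle and movement animation.
; Separate start and stop events control two timelines, one for idle and one for movement.
; Each timeline's Squash and Rotation tracks drive lerps of the mesh's relative scale and rotation, producing squash-and-stretch with a slight tilt.
; Stopping a timeline does not reset the mesh transform, and existing notes label the motions as vehicle idle and car movement.
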(event Custom|DAnimal%20Stop%20Movement
  (bind _creaturemesh (Variables|Default|GetCreatureMesh))
  ;[1 1 1] car movement
  (bind (_direction _squash _rotation) (Timeline|Timeline_1 Stop)
    (:Update
      (Transformation|SetRelativeScale3D _creaturemesh (Math|Vector|Lerp(Vector) "1.000000,1.000000,1.000000" "1.050000,1.050000,0.950000" _squash))
      (Transformation|SetRelativeRotation _creaturemesh (Math|Rotator|Lerp(Rotator) "0, 0, 0" "-5.000000, 0,0.000000" _rotation) false false))))

(event Custom|DAnimal%20stop%20idle
  (bind _creaturemesh (Variables|Default|GetCreatureMesh))
  ;[1 1 1] vehicle idle (use on both tanks and cars)
  (bind (_direction _squash _rotation) (Timeline|Timeline_0 Stop)
    (:Update
      (Transformation|SetRelativeScale3D _creaturemesh (Math|Vector|Lerp(Vector) "1.000000,1.000000,1.000000" "1.050000,1.050000,0.950000" _squash))
      (Transformation|SetRelativeRotation _creaturemesh (Math|Rotator|Lerp(Rotator) "5.000000, 0,0.000000" "0, 0, 0" _rotation) false false))))

(event Custom|DAnimal%20start%20idle
  (bind _creaturemesh (Variables|Default|GetCreatureMesh))
  ;[1 1 1] vehicle idle (use on both tanks and cars)
  (bind (_direction _squash _rotation) (Timeline|Timeline_0 PlayFromStart)
    (:Update
      (Transformation|SetRelativeScale3D _creaturemesh (Math|Vector|Lerp(Vector) "1.000000,1.000000,1.000000" "1.050000,1.050000,0.950000" _squash))
      (Transformation|SetRelativeRotation _creaturemesh (Math|Rotator|Lerp(Rotator) "5.000000, 0,0.000000" "0, 0, 0" _rotation) false false))))

(event Custom|DAnimal%20Start%20Movement
  (bind _creaturemesh (Variables|Default|GetCreatureMesh))
  ;[1 1 1] car movement
  (bind (_direction _squash _rotation) (Timeline|Timeline_1 PlayFromStart)
    (:Update
      (Transformation|SetRelativeScale3D _creaturemesh (Math|Vector|Lerp(Vector) "1.000000,1.000000,1.000000" "1.050000,1.050000,0.950000" _squash))
      (Transformation|SetRelativeRotation _creaturemesh (Math|Rotator|Lerp(Rotator) "0, 0, 0" "-5.000000, 0,0.000000" _rotation) false false))))

(fn ConstructionScript)