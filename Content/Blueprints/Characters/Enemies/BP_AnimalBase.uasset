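; BP_AnimalBase is the base creature Blueprint, providing procedural idle and walk animation through start and stop events.
; Timelines drive CreatureMesh transforms instead of skeletal animation: idle is a subtle squash and sway, which ghosts also use as movement.
; Walking hops and squashes the mesh, with a nested timeline played from its update adding a pitch tilt.
; Stop events halt only the main idle or walk timeline, without resetting the mesh transform.
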(event Custom|Animal%20Stop%20Movement
  (bind _creaturemesh (Variables|Default|GetCreatureMesh))
  ;[1 1 1] Walking movement
  (bind (_direction _jump _squash) (Timeline|Timeline_0 Stop)
    (:Update
      (Transformation|SetRelativeLocation _creaturemesh (Math|Vector|Lerp(Vector) "0, 0, 0" "0.000000,0.000000,60.000000" _jump) false false)
      (Transformation|SetRelativeScale3D _creaturemesh (Math|Vector|Lerp(Vector) "1.000000,1.000000,1.000000" "1.400000,1.400000,0.600000" _squash))
      (bind _rotation (Timeline|Timeline_1 Play)
        (:Update
          (Transformation|SetRelativeRotation _creaturemesh (Math|Rotator|Lerp(Rotator) "0, 0, 0" "0.000000, 0,10.000000" _rotation) false false))))))

(event Custom|Animal%20stop%20idle
  (bind _creaturemesh (Variables|Default|GetCreatureMesh))
  ;[1 1 1] idle movement (all creatures gets this, ghosts use this a movement too)
  (bind (_direction _squash _rotation) (Timeline|Timeline_2 Stop)
    (:Update
      (Transformation|SetRelativeScale3D _creaturemesh (Math|Vector|Lerp(Vector) "1.000000,1.000000,1.000000" "1.100000,1.100000,0.900000" _squash))
      (Transformation|SetRelativeRotation _creaturemesh (Math|Rotator|Lerp(Rotator) "0, 0, 0" "2.000000,0.000000,0.000000" _rotation) false false))))

(event Custom|Animal%20start%20idle
  (bind _creaturemesh (Variables|Default|GetCreatureMesh))
  ;[1 1 1] idle movement (all creatures gets this, ghosts use this a movement too)
  (bind (_direction _squash _rotation) (Timeline|Timeline_2 PlayFromStart)
    (:Update
      (Transformation|SetRelativeScale3D _creaturemesh (Math|Vector|Lerp(Vector) "1.000000,1.000000,1.000000" "1.100000,1.100000,0.900000" _squash))
      (Transformation|SetRelativeRotation _creaturemesh (Math|Rotator|Lerp(Rotator) "0, 0, 0" "2.000000,0.000000,0.000000" _rotation) false false))))

(event Custom|Animal%20Start%20Movement
  (bind _creaturemesh (Variables|Default|GetCreatureMesh))
  ;[1 1 1] Walking movement
  (bind (_direction _jump _squash) (Timeline|Timeline_0 PlayFromStart)
    (:Update
      (Transformation|SetRelativeLocation _creaturemesh (Math|Vector|Lerp(Vector) "0, 0, 0" "0.000000,0.000000,60.000000" _jump) false false)
      (Transformation|SetRelativeScale3D _creaturemesh (Math|Vector|Lerp(Vector) "1.000000,1.000000,1.000000" "1.400000,1.400000,0.600000" _squash))
      (bind _rotation (Timeline|Timeline_1 Play)
        (:Update
          (Transformation|SetRelativeRotation _creaturemesh (Math|Rotator|Lerp(Rotator) "0, 0, 0" "0.000000, 0,10.000000" _rotation) false false))))))

(fn ConstructionScript)