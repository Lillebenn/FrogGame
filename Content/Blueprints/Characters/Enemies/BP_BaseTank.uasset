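; Base tank enemy that fires projectiles and fakes shooting and movement animation procedurally on its creature mesh.
; BeginPlay attaches an optional ambient sound to the capsule.
; StartShooting resets mesh rotation, spawns a Tank_Projectile at the barrel exit, plays any shoot sound and runs a squash-and-rotate recoil timeline.
; StartMoving runs a second, gentler squash-and-rotate timeline, which StopMoving halts in place.
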(event Custom|StartShooting
  (bind _returnvalue (Class|SimpleCreature|GetShootSound))
  (bind _creaturemesh (Variables|Default|GetCreatureMesh))
  (Transformation|SetRelativeRotation (Variables|Default|GetCreatureMesh) "0, 0, 0" false false)
  (Game|SpawnActorfromClass "/Game/Blueprints/Characters/Enemies/Tank_Projectile.Tank_Projectile_C" (Transformation|GetSocketTransform (Variables|Default|GetBarrelExit) "None" "RTS_World") "Undefined" 0 0)
  (Utilities|IsValid _returnvalue
    (:Is%20Valid
      ;[1 1 1] tank shoot
      (Audio|PlaySoundatLocation _returnvalue (Transformation|GetWorldLocation (Variables|Default|GetBarrelExit)) "0, 0, 0" 1.0 1.0 0.0 0 0 0)
      (bind (_direction _squash _rotation) (Timeline|Timeline_0 PlayFromStart)
        (:Update
          (Transformation|SetRelativeScale3D _creaturemesh (Math|Vector|Lerp(Vector) "1.000000,1.000000,1.000000" "1.100000,1.100000,0.900000" _squash))
          (Transformation|SetRelativeRotation _creaturemesh (Math|Rotator|Lerp(Rotator) "5.000000,0.000000,0.000000" "20.000000,0.000000,0.000000" _rotation) false false))))
    (:Is%20Not%20Valid
      (Timeline|Timeline_0 PlayFromStart))))

(event Custom|StartMoving
  (bind _creaturemesh (Variables|Default|GetCreatureMesh))
  ;[1 1 1] tank movement
  (bind (_direction _jump _squash _rotation) (Timeline|Timeline_1 PlayFromStart)
    (:Update
      (Transformation|SetRelativeScale3D _creaturemesh (Math|Vector|Lerp(Vector) "1.000000,1.000000,1.000000" "1.100000,1.100000,0.900000" _squash))
      (Transformation|SetRelativeRotation _creaturemesh (Math|Rotator|Lerp(Rotator) "5.000000,0.000000,0.000000" "10.000000,0.000000,0.000000" _rotation) false false))))

(event Custom|Stop%20Moving
  (bind _creaturemesh (Variables|Default|GetCreatureMesh))
  ;[1 1 1] tank movement
  (bind (_direction _jump _squash _rotation) (Timeline|Timeline_1 Stop)
    (:Update
      (Transformation|SetRelativeScale3D _creaturemesh (Math|Vector|Lerp(Vector) "1.000000,1.000000,1.000000" "1.100000,1.100000,0.900000" _squash))
      (Transformation|SetRelativeRotation _creaturemesh (Math|Rotator|Lerp(Rotator) "5.000000,0.000000,0.000000" "10.000000,0.000000,0.000000" _rotation) false false))))

(event EventBeginPlay
  (bind _ambientsound (Variables|Default|GetAmbientSound))
  (Utilities|IsValid _ambientsound
    (:Is%20Valid
      (Audio|SpawnSoundAttached _ambientsound (Variables|Default|GetCapsuleComponent) "None" "0, 0, 0" "0, 0, 0" "KeepRelativeOffset" false 1.0 1.0 0.0 0 0))))

(fn ConstructionScript)