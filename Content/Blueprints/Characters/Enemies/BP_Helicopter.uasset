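; BP_Helicopter is an enemy helicopter character that fires missiles.
; Its HelicopterShooting event zeroes the creature mesh's relative rotation, then spawns a Helicopter_Missile at a launcher's world transform.
; The MissileLauncher flag selects the right launcher when true and the left when false.
; This graph neither toggles that flag nor calls the event.
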(event Custom|HelicopterShooting
  (if (Variables|Default|GetMissileLauncher)
    (Transformation|SetRelativeRotation (Variables|Default|GetCreatureMesh) "0, 0, 0" false false)
    (Game|SpawnActorfromClass "/Game/Blueprints/Characters/Enemies/Helicopter_Missile.Helicopter_Missile_C" (Transformation|GetSocketTransform (Variables|Default|GetRightMissileLauncher) "None" "RTS_World") "Undefined" 0 0)
    (else
      (Transformation|SetRelativeRotation (Variables|Default|GetCreatureMesh) "0, 0, 0" false false)
      (Game|SpawnActorfromClass "/Game/Blueprints/Characters/Enemies/Helicopter_Missile.Helicopter_Missile_C" (Transformation|GetSocketTransform (Variables|Default|GetLeftMissileLauncher) "None" "RTS_World") "Undefined" 0 0))))

(fn ConstructionScript)