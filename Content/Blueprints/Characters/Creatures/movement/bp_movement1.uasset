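; Test-bed actor of procedural squash-and-stretch animations for creatures and vehicles, made with timelines that lerp a StaticMesh's relative transform.
; Only the "getting sucked" animation runs, from BeginPlay: it squashes the mesh while a nested timeline adds a full spin plus tilt; its location lerp stays at zero.
; Unconnected presets cover idle, walking, driving, boat bobbing, flying and shooting, some nesting a second timeline for rotation.
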(event EventBeginPlay
  (bind _static_mesh (Variables|Default|Getstatic_mesh))
  ;[1 1 1] getting sucked
  (bind (_direction _jump _squash _rotation) (Timeline|Timeline_12 Play)
    (:Update
      (Transformation|SetRelativeLocation _static_mesh (Math|Vector|Lerp(Vector) "0, 0, 0" "0, 0, 0" _jump) false false)
      (Transformation|SetRelativeScale3D _static_mesh (Math|Vector|Lerp(Vector) "1.000000,1.000000,1.000000" "1.200000,1.200000,0.800000" _squash))
      (bind _rotation_2 (Timeline|Timeline_13 Play)
        (:Update
          (Transformation|SetRelativeRotation _static_mesh (Math|Rotator|Lerp(Rotator) "0, 0, 0" "0.000000,360.000000,0.000000" _rotation_2) false false)
          (Transformation|AddRelativeRotation _static_mesh (Math|Rotator|Lerp(Rotator) "0, 0, 0" "0.000000,0.000000,10.000000" _rotation) false false))))))

(event Collision|EventActorBeginOverlap
  (params (OtherActor :type Actor%20Object%20Reference)))

(event EventTick
  (params (DeltaSeconds :type Float%20%28single-precision%29)))

(fn ConstructionScript)