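; Movement Blueprint that fakes animation on a static mesh with procedural squash-and-tilt motion, apparently a backup copy.
; On BeginPlay a timeline plays the tank movement preset, using its Squash and Rotation tracks to lerp the mesh's relative scale and rotation.
; Unconnected timeline variants for tank movement, vehicle idle, walking with a hop, idle and tank shoot remain in the graph but never run.
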(event EventBeginPlay
  (bind _static_mesh (Variables|Default|Getstatic_mesh))
  ;[1 1 1] tank movement
  (bind (_direction _jump _squash _rotation) (Timeline|Timeline_3 Play)
    (:Update
      (Transformation|SetRelativeScale3D _static_mesh (Math|Vector|Lerp(Vector) "1.000000,1.000000,1.000000" "1.100000,1.100000,0.900000" _squash))
      (Transformation|SetRelativeRotation _static_mesh (Math|Rotator|Lerp(Rotator) "0, 0,-5.000000" "0.000000, 0,-10.000000" _rotation) false false))))

(event Collision|EventActorBeginOverlap
  (params (OtherActor :type Actor%20Object%20Reference)))

(event EventTick
  (params (DeltaSeconds :type Float%20%28single-precision%29)))

(fn ConstructionScript)