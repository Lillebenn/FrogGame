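; In-game indicator arrow actor that plays a bobbing, spinning animation above the SkNormalMale component's position.
; On BeginPlay a timeline drives Arrow1's world height offset, squash-and-stretch scale and full-turn yaw through lerps.
; BeginPlay also sets Cube as the component updated by RotatingMovement.
; An additional rotation step on Arrow1 is left disconnected and never runs.
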(event EventBeginPlay
  (bind _arrow1 (Variables|Default|Getarrow1))
  (Components|Movement|SetUpdatedComponent (Variables|Default|GetRotatingMovement) (Variables|Default|GetCube))
  ;[1 1 1] arrow loop anim
  (bind (_direction _position _scale _rotation _rotation_2) (Timeline|Timeline_0 PlayFromStart)
    (:Update
      (Transformation|SetWorldLocation _arrow1 (+ (Transformation|GetWorldLocation (Variables|Default|Getsk_normal_male)) (Math|Vector|Lerp(Vector) "0, 0,400.000000" "0, 0,200.000000" _position)) false false)
      (Transformation|SetRelativeScale3D _arrow1 (Math|Vector|Lerp(Vector) "1.000000,1.000000,1.000000" "1.200000,1.200000,0.800000" _scale))
      (Transformation|SetRelativeRotation _arrow1 (Math|Rotator|Lerp(Rotator) "0.000000, 0,0.000000" "0.000000,360.000000,0.000000" _rotation) false false))))

(event Collision|EventActorBeginOverlap
  (params (OtherActor :type Actor%20Object%20Reference)))

(event EventTick
  (params (DeltaSeconds :type Float%20%28single-precision%29)))

(fn ConstructionScript)