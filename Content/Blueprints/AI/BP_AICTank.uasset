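; AI controller for tank enemies that runs the BT_Tank behavior tree and reacts to sighting the frog player.
; On BeginPlay it copies the controlled tank's patrol path looping flag and wait time into the blackboard, along with an initial patrol direction.
; AI perception updates for BP_FrogCharacter set or clear the CanTankSeePlayer blackboard key, leaving behavior decisions to the tree.
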(event OnTargetPerceptionUpdated(AIPerception)
  (params (Actor :type Actor%20Object%20Reference) (Stimulus :type AI%20Stimulus%20Structure))
  (bind _bsuccessfullysensed (Utilities|Struct|BreakAIStimulus Stimulus))
  (bind _returnvalue (Utilities|Name|MakeLiteralName "CanTankSeePlayer"))
  (bind _returnvalue_2 (AI|GetBlackboard 0))
  (Utilities|Casting|CastToBP_FrogCharacter Actor)
  (if _bsuccessfullysensed
    (AI|Components|Blackboard|SetValueasBool _returnvalue_2 _returnvalue _bsuccessfullysensed)
    (else
      (AI|Components|Blackboard|SetValueasBool _returnvalue_2 _returnvalue false))))

(event EventBeginPlay
  (bind _returnvalue (AI|GetBlackboard 0))
  (AI|RunBehaviorTree "/Game/Blueprints/AI/BT_Tank.BT_Tank")
  (bind _astank (Utilities|Casting|CastToTank (Pawn|GetControlledPawn)))
  (bind _output_get (Variables|Default|SetMyPawn _astank))
  (AI|Components|Blackboard|SetValueasBool _returnvalue (Utilities|Name|MakeLiteralName "TankPathLooping") (Variables|/Game/Blueprints/Characters/Enemies/PatrolPath.PatrolPath_C|GetIsLooping (Variables|/Game/Blueprints/Characters/Enemies/Tank.Tank_C|GetPatrolPath _output_get)))
  (Class|BlackboardComponent|SetValueasInt _returnvalue (Utilities|Name|MakeLiteralName "TankDirection") 1)
  (AI|Components|Blackboard|SetValueasFloat _returnvalue (Utilities|Name|MakeLiteralName "TankWaitTime") (Variables|/Game/Blueprints/Characters/Enemies/PatrolPath.PatrolPath_C|GetWaitTime (Variables|/Game/Blueprints/Characters/Enemies/Tank.Tank_C|GetPatrolPath (Variables|Default|GetMyPawn)))))

(fn ConstructionScript)