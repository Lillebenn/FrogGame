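; Behavior tree task that picks the next patrol point for a directional animal AI.
; It stops the animal, then converts the patrol path point at the blackboard's path index from the path actor's local space to world space.
; It writes that location to the blackboard, starts the animal's idle and finishes successfully.
; Without a valid patrol path or matching pawn, the task never calls finish.
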(event EventReceiveExecuteAI
  (params (OwnerController :type AI%20Controller%20Object%20Reference) (ControlledPawn :type Pawn%20Object%20Reference))
  (bind _asbp_directional_animal (Utilities|Casting|CastToBP_DirectionalAnimal ControlledPawn))
  (Default|DAnimalStopMovement _asbp_directional_animal)
  (bind _patrolpath (Variables|/Game/Blueprints/Characters/Enemies/BP_DirectionalAnimal.BP_DirectionalAnimal_C|GetPatrolPath _asbp_directional_animal)
    (:then
      (AI|BehaviorTree|SetBlackboardValueasVector (Variables|Default|GetBB_PathVector) (Math|Transform|TransformLocation (Transformation|GetActorTransform _patrolpath) (Utilities|Array|Get(acopy) (Variables|/Game/Blueprints/Characters/Enemies/PatrolPath.PatrolPath_C|GetPathPoints _patrolpath) (Class|BTFunctionLibrary|GetBlackboardValueasInt (Variables|Default|GetBB_PathIndex)))))
      (Default|DAnimalStartIdle _asbp_directional_animal)
      (AI|BehaviorTree|FinishExecute true))
    (:else)))