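; Behavior tree task that smoothly turns the controlled pawn to face a location stored in a blackboard vector key.
; Each AI tick it computes the look-at rotation toward that point and interpolates the pawn's yaw toward it at a configurable rotation rate.
; The task finishes successfully once the interpolated yaw is within one degree of the target yaw.
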(event EventReceiveTickAI
  (params (OwnerController :type AI%20Controller%20Object%20Reference) (ControlledPawn :type Pawn%20Object%20Reference) (DeltaSeconds :type Float%20%28single-precision%29))
  (bind _output_get (Variables|Default|SetControlled%20Pawn ControlledPawn))
  (Transformation|SetActorRotation (Variables|Default|GetControlled%20Pawn) (Math|Interpolation|RInterpTo (Math|Rotator|MakeRotator 0.0 0.0 (.yaw (Transformation|GetActorRotation _output_get))) (Math|Rotator|MakeRotator 0.0 0.0 (.yaw (Math|Rotator|FindLookatRotation (Transformation|GetActorLocation (Variables|Default|GetControlled%20Pawn)) (Class|BTFunctionLibrary|GetBlackboardValueasVector (Variables|Default|GetBB_PathVector))))) DeltaSeconds (Variables|Default|GetRotation%20Rate)))
  (if (and (< (.yaw (Math|Rotator|Delta(Rotator) (Math|Interpolation|RInterpTo (Math|Rotator|MakeRotator 0.0 0.0 (.yaw (Transformation|GetActorRotation _output_get))) (Math|Rotator|MakeRotator 0.0 0.0 (.yaw (Math|Rotator|FindLookatRotation (Transformation|GetActorLocation (Variables|Default|GetControlled%20Pawn)) (Class|BTFunctionLibrary|GetBlackboardValueasVector (Variables|Default|GetBB_PathVector))))) DeltaSeconds (Variables|Default|GetRotation%20Rate)) (Math|Rotator|MakeRotator (.roll (Math|Rotator|FindLookatRotation (Transformation|GetActorLocation (Variables|Default|GetControlled%20Pawn)) (Class|BTFunctionLibrary|GetBlackboardValueasVector (Variables|Default|GetBB_PathVector)))) (.pitch (Math|Rotator|FindLookatRotation (Transformation|GetActorLocation (Variables|Default|GetControlled%20Pawn)) (Class|BTFunctionLibrary|GetBlackboardValueasVector (Variables|Default|GetBB_PathVector)))) (.yaw (Math|Rotator|FindLookatRotation (Transformation|GetActorLocation (Variables|Default|GetControlled%20Pawn)) (Class|BTFunctionLibrary|GetBlackboardValueasVector (Variables|Default|GetBB_PathVector))))))) 1.0) (> (.yaw (Math|Rotator|Delta(Rotator) (Math|Interpolation|RInterpTo (Math|Rotator|MakeRotator 0.0 0.0 (.yaw (Transformation|GetActorRotation _output_get))) (Math|Rotator|MakeRotator 0.0 0.0 (.yaw (Math|Rotator|FindLookatRotation (Transformation|GetActorLocation (Variables|Default|GetControlled%20Pawn)) (Class|BTFunctionLibrary|GetBlackboardValueasVector (Variables|Default|GetBB_PathVector))))) DeltaSeconds (Variables|Default|GetRotation%20Rate)) (Math|Rotator|MakeRotator (.roll (Math|Rotator|FindLookatRotation (Transformation|GetActorLocation (Variables|Default|GetControlled%20Pawn)) (Class|BTFunctionLibrary|GetBlackboardValueasVector (Variables|Default|GetBB_PathVector)))) (.pitch (Math|Rotator|FindLookatRotation (Transformation|GetActorLocation (Variables|Default|GetControlled%20Pawn)) (Class|BTFunctionLibrary|GetBlackboardValueasVector (Variables|Default|GetBB_PathVector)))) (.yaw (Math|Rotator|FindLookatRotation (Transformation|GetActorLocation (Variables|Default|GetControlled%20Pawn)) (Class|BTFunctionLibrary|GetBlackboardValueasVector (Variables|Default|GetBB_PathVector))))))) -1.0))
    (AI|BehaviorTree|FinishExecute true)))