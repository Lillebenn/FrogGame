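; Behavior tree task that gives an AdvCreature pawn its next patrol destination.
; It reads the path index from the blackboard and picks that entry from the creature's PatrolSettings path points.
; The point is transformed from local to world space by the pawn's current transform, then written to the blackboard path vector.
; The task fails when the index reaches the point count, and never finishes if the cast fails.
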(event EventReceiveExecuteAI
  (params (OwnerController :type AI%20Controller%20Object%20Reference) (ControlledPawn :type Pawn%20Object%20Reference))
  (bind _bb_pathindex (Variables|Default|GetBB_PathIndex))
  (bind _returnvalue (Class|BTFunctionLibrary|GetBlackboardValueasInt _bb_pathindex))
  (bind _asadv_creature (Utilities|Casting|CastToAdvCreature ControlledPawn))
  (if (< _returnvalue (Utilities|Array|Length (.pathpoints (Variables|/Script/FrogGame.AdvCreature|GetPatrolSettings _asadv_creature))))
    (AI|BehaviorTree|SetBlackboardValueasVector (Variables|Default|GetBB_PathVector) (Math|Transform|TransformLocation (Transformation|GetActorTransform ControlledPawn) (Utilities|Array|Get(acopy) (.pathpoints (Variables|/Script/FrogGame.AdvCreature|GetPatrolSettings _asadv_creature)) _returnvalue)))
    (AI|BehaviorTree|FinishExecute true)
    (else
      (AI|BehaviorTree|FinishExecute false))))