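; Behavior tree task that turns an animal's CreatureMesh to align with its movement during AI behavior.
; On execute, it builds a rotation from the pawn's negated, normalized velocity, applies one RInterpToConstant step to the mesh's world rotation, then finishes.
; The step reads DeltaSeconds from the otherwise empty tick event.
; An unconnected alternative rotates the actor toward the current patrol path point.
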(event EventReceiveExecuteAI
  (params (OwnerController :type AI%20Controller%20Object%20Reference) (ControlledPawn :type Pawn%20Object%20Reference))
  (bind _returnvalue (Transformation|GetVelocity ControlledPawn))
  (bind _returnvalue_2 (Math|Vector|Normalize _returnvalue))
  (bind _returnvalue_3 (* _returnvalue_2 -1.0))
  (bind _returnvalue_4 (Math|Conversions|RotationFromXVector _returnvalue_3))
  (bind _asbp_animal_base (Utilities|Casting|CastToBP_AnimalBase ControlledPawn))
  (Transformation|SetWorldRotation (Variables|/Script/FrogGame.SimpleCreature|GetCreatureMesh _asbp_animal_base) (Class|KismetMathLibrary|RInterptoConstant (Transformation|GetWorldRotation (Variables|/Script/FrogGame.SimpleCreature|GetCreatureMesh _asbp_animal_base)) (Math|Rotator|MakeRotationfromAxes (Math|Vector|GetForwardVector _returnvalue_4) (Math|Vector|GetRightVector _returnvalue_4) "0, 0,1.000000") (stale EventReceiveTickAI DeltaSeconds) 3.6e+02) false false)
  (AI|BehaviorTree|FinishExecute true))

(event EventReceiveTickAI
  (params (OwnerController :type AI%20Controller%20Object%20Reference) (ControlledPawn :type Pawn%20Object%20Reference) (DeltaSeconds :type Float%20%28single-precision%29)))