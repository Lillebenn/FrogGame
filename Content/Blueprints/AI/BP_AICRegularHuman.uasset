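; AI controller for regular human NPCs that runs the BT_RegularHuman behavior tree.
; On BeginPlay it casts the controlled pawn to RegularHuman and stores it.
; It then seeds the blackboard with the looping flag and wait time from the pawn's assigned patrol path, plus an initial forward direction for patrolling.
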(event EventBeginPlay
  (bind _returnvalue (AI|GetBlackboard 0))
  (AI|RunBehaviorTree "/Game/Blueprints/AI/BT_RegularHuman.BT_RegularHuman")
  (bind _asregular_human (Utilities|Casting|CastToRegularHuman (Pawn|GetControlledPawn)))
  (bind _output_get (Variables|Default|SetMyPawn _asregular_human))
  (AI|Components|Blackboard|SetValueasBool _returnvalue (Utilities|Name|MakeLiteralName "PathLooping") (Variables|/Game/Blueprints/Characters/Enemies/PatrolPath.PatrolPath_C|GetIsLooping (Variables|/Game/Blueprints/Characters/Enemies/RegularHuman.RegularHuman_C|GetPatrolPath _output_get)))
  (Class|BlackboardComponent|SetValueasInt _returnvalue (Utilities|Name|MakeLiteralName "Direction") 1)
  (AI|Components|Blackboard|SetValueasFloat _returnvalue (Utilities|Name|MakeLiteralName "WaitTime") (Variables|/Game/Blueprints/Characters/Enemies/PatrolPath.PatrolPath_C|GetWaitTime (Variables|/Game/Blueprints/Characters/Enemies/RegularHuman.RegularHuman_C|GetPatrolPath (Variables|Default|GetMyPawn)))))

(fn ConstructionScript)