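; Behavior tree task that gives an animal AI the next destination on its assigned patrol path.
; It stops the animal's movement, then reads the current path index from the blackboard and converts that path point from the patrol actor's local space to world space.
; It writes the result to a blackboard vector, starts the animal's idle and finishes successfully.
; The task only finishes when the cast succeeds and a valid patrol path exists.
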(event EventReceiveExecuteAI
  (params (OwnerController :type AI%20Controller%20Object%20Reference) (ControlledPawn :type Pawn%20Object%20Reference))
  (bind _asbp_animal_base (Utilities|Casting|CastToBP_AnimalBase ControlledPawn))
  (Default|AnimalStopMovement _asbp_animal_base)
  (bind _patrolpath (Variables|/Game/Blueprints/Characters/Enemies/BP_AnimalBase.BP_AnimalBase_C|GetPatrolPath _asbp_animal_base)
    (:then
      (AI|BehaviorTree|SetBlackboardValueasVector (Variables|Default|GetBB_PathVector) (Math|Transform|TransformLocation (Transformation|GetActorTransform _patrolpath) (Utilities|Array|Get(acopy) (Variables|/Game/Blueprints/Characters/Enemies/PatrolPath.PatrolPath_C|GetPathPoints _patrolpath) (Class|BTFunctionLibrary|GetBlackboardValueasInt (Variables|Default|GetBB_PathIndex)))))
      (Default|AnimalStartIdle _asbp_animal_base)
      (AI|BehaviorTree|FinishExecute true))
    (:else)))