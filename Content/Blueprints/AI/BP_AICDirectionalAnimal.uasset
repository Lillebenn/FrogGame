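; AI controller for the directional animal pawn, which starts its behavior tree when play begins.
; It casts the controlled pawn to BP_DirectionalAnimal, stores it, and copies the looping flag and wait time from that pawn's patrol path into the blackboard.
; It also seeds an initial forward direction value in the blackboard alongside those patrol settings.
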(event EventBeginPlay
  (bind _returnvalue (AI|GetBlackboard 0))
  (AI|RunBehaviorTree "/Game/Blueprints/AI/BT_DirectionalAnimal.BT_DirectionalAnimal")
  (bind _asbp_directional_animal (Utilities|Casting|CastToBP_DirectionalAnimal (Pawn|GetControlledPawn)))
  (bind _output_get (Variables|Default|SetMyPawn _asbp_directional_animal))
  (AI|Components|Blackboard|SetValueasBool _returnvalue (Utilities|Name|MakeLiteralName "DAPathLooping") (Variables|/Game/Blueprints/Characters/Enemies/PatrolPath.PatrolPath_C|GetIsLooping (Variables|/Game/Blueprints/Characters/Enemies/BP_DirectionalAnimal.BP_DirectionalAnimal_C|GetPatrolPath _output_get)))
  (Class|BlackboardComponent|SetValueasInt _returnvalue (Utilities|Name|MakeLiteralName "DADirection") 1)
  (AI|Components|Blackboard|SetValueasFloat _returnvalue (Utilities|Name|MakeLiteralName "DAWaitTime") (Variables|/Game/Blueprints/Characters/Enemies/PatrolPath.PatrolPath_C|GetWaitTime (Variables|/Game/Blueprints/Characters/Enemies/BP_DirectionalAnimal.BP_DirectionalAnimal_C|GetPatrolPath (Variables|Default|GetMyPawn)))))

(fn ConstructionScript)