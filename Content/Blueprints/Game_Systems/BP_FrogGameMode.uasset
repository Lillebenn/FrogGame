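; Game mode for the frog game that manages background music and relays main menu and end-of-run events.
; Power, regular and main menu tracks each spawn as 2D sounds on first play and are reused afterwards, with regular music starting on BeginPlay.
; PauseMusic checks the frog character's PowerMode to choose which track to pause or resume.
; Opening the main menu and reaching the swamp fire event dispatchers, and the swamp also pauses the music.
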(event Custom|Play%20PowerMode
  (params (ShouldPlay :type Boolean))
  ;[1 1 1] Power Mode Music
  (Utilities|IsValid (Variables|Default|GetPowerModeAudio)
    (:Is%20Valid
      (if ShouldPlay
        (Audio|Components|Audio|Play (Variables|Default|GetPowerModeAudio) 0.0)
        (else
          (Audio|Components|Audio|Stop (Variables|Default|GetPowerModeAudio)))))
    (:Is%20Not%20Valid
      (if ShouldPlay
        (bind _returnvalue (Audio|SpawnSound2D "/Game/sound/music/mfx_powered_frog.mfx_powered_frog" 1.0 1.0 0.0 0))
        (Variables|Default|SetPowerModeAudio _returnvalue)))))

(event Custom|Play%20RegularMode
  (params (ShouldPlay :type Boolean))
  ;[1 1 1] Regular Mode Music
  (Utilities|IsValid (Variables|Default|GetRegularModeAudio)
    (:Is%20Valid
      (if ShouldPlay
        (Audio|Components|Audio|Play (Variables|Default|GetRegularModeAudio) 0.0)
        (else
          (Audio|Components|Audio|Stop (Variables|Default|GetRegularModeAudio)))))
    (:Is%20Not%20Valid
      (if ShouldPlay
        (bind _returnvalue (Audio|SpawnSound2D "/Game/sound/music/mfx_regular_forg.mfx_regular_forg" 1.0 1.0 0.0 0))
        (Variables|Default|SetRegularModeAudio _returnvalue)))))

(event Custom|Play%20Main%20Menu
  (params (ShouldPlay :type Boolean))
  ;[1 1 1] Start Main Menu music
  (Utilities|IsValid (Variables|Default|GetMainMenuAudio)
    (:Is%20Valid
      (if ShouldPlay
        (Audio|Components|Audio|Play (Variables|Default|GetMainMenuAudio) 0.0)
        (else
          (Audio|Components|Audio|Stop (Variables|Default|GetMainMenuAudio)))))
    (:Is%20Not%20Valid
      (if ShouldPlay
        (bind _returnvalue (Audio|SpawnSound2D "/Game/sound/music/mfx_main_menu.mfx_main_menu" 1.0 1.0 0.0 0))
        (Variables|Default|SetMainMenuAudio _returnvalue)))))

(event Custom|PauseMusic
  (params (ShouldPause :type Boolean))
  (bind _asbp_frog_character (Utilities|Casting|CastToBP_FrogCharacter (Game|GetPlayerCharacter 0)))
  (if ShouldPause
    ;[1 1 1] Pause Music
    (if (Variables|/Script/FrogGame.FrogGameCharacter|GetbPowerMode _asbp_frog_character)
      (Class|AudioComponent|SetPaused (Variables|Default|GetPowerModeAudio) true)
      (else
        (Class|AudioComponent|SetPaused (Variables|Default|GetRegularModeAudio) true)))
    (else
      ;[1 1 1] Restart music
      (if (Variables|/Script/FrogGame.FrogGameCharacter|GetbPowerMode _asbp_frog_character)
        (Class|AudioComponent|SetPaused (Variables|Default|GetPowerModeAudio) false)
        (else
          (Class|AudioComponent|SetPaused (Variables|Default|GetRegularModeAudio) false))))))

(event EventOpenedMainMenu
  (Default|CallSetViewMainMenu))

(event EventTick
  (params (DeltaSeconds :type Float%20%28single-precision%29)))

(event EventBeginPlay
  (CallFunction|PlayRegularMode true))

(event EventReachedSwamp
  (Default|CallStartEndSequence)
  (CallFunction|PauseMusic true))

(fn ConstructionScript)