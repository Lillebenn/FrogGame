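; Particle-testing Blueprint for a shatter mesh that animates itself into place when spawned.
; On BeginPlay, a timeline raises the mesh from below its origin while a separate track blends its scale toward a wide, flattened squash shape.
; A mirrored despawn timeline lowers it again but is never triggered.
; Random spawn rotation and per-axis random scale are unfinished and unconnected.
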(event EventBeginPlay
  (bind _mesh (Variables|Default|Getmesh))
  ;[1 1 1] spawn anim
  (bind (_direction _position _scale) (Timeline|Timeline_0 PlayFromStart)
    (:Update
      (Transformation|SetRelativeLocation _mesh (Math|Vector|Lerp(Vector) "0.000000, 0,-260.000000" "0.000000,0.000000,0.000000" _position) false false)
      (Transformation|SetRelativeScale3D _mesh (Math|Vector|Lerp(Vector) "1.000000,1.000000,1.000000" "1.400000,1.400000,0.600000" _scale)))))

(fn ConstructionScript)